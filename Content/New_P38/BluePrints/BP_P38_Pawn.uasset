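; BP_P38_Pawn is a player-controlled P-38 aircraft pawn with simple arcade-style flight and no yaw control.
; Roll and Pitch axis inputs rotate the actor directly in local space.
; Acceleration and Deceleration axes adjust a clamped MoveSpeed between zero and MaxMoveSpeed.
; Tick moves the pawn along its local forward axis by MoveSpeed, without delta-time scaling, so movement depends on frame rate.
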(event `InputAxis|Roll`
  (params (AxisValue :type "Float (single-precision)"))
  (`self.K2_AddActorLocalRotation` (`KismetMathLibrary.MakeRotator` AxisValue)))

(event `InputAxis|Pitch`
  (params (AxisValue :type "Float (single-precision)"))
  (`self.K2_AddActorLocalRotation` (`KismetMathLibrary.MakeRotator` 0.0 AxisValue)))

(event `self.ReceiveTick`
  (params (DeltaSeconds :type "Float (single-precision)"))
  (`self.K2_AddActorLocalOffset` (`KismetMathLibrary.MakeVector` (`self.MoveSpeed`))))

(event `InputAxis|Acceleration`
  (params (AxisValue :type "Float (single-precision)"))
  (set `self.MoveSpeed` (`KismetMathLibrary.FClamp` (+ (* AxisValue (`self.Acceleration`)) (`self.MoveSpeed`)) 0.0 (`self.MaxMoveSpeed`))))

(event `InputAxis|Deceleration`
  (params (AxisValue :type "Float (single-precision)"))
  (set `self.MoveSpeed` (`KismetMathLibrary.FClamp` (- (`self.MoveSpeed`) (* AxisValue (`self.Acceleration`))) 0.0 (`self.MaxMoveSpeed`))))

(fn `UserConstructionScript`)
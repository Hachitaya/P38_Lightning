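; BP_Rocket is a homing rocket projectile that explodes on overlap with any actor other than BP_P38_Pawn.
; On BeginPlay it sets its lifespan and loops over all "Enemy"-tagged actors, assigning each root as the ProjectileMovement homing target, so the last one found wins regardless of distance.
; On a qualifying overlap it spawns an explosion emitter and destroys itself, without applying damage.
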(event `self.ReceiveBeginPlay`
  (`|ExecutionSequence`
    (:`then_0`
      (`self.SetLifeSpan` (`self.RocketLifeSpan`)))
    (:`then_1`
      (bind _outactors (`GameplayStatics.GetAllActorsWithTag` "Enemy"))
      (for _array_element _outactors
        (set `ProjectileMovementComponent.HomingTargetComponent` (`Actor.RootComponent` _array_element) (`self.ProjectileMovement`))))))

(event `self.ReceiveActorBeginOverlap`
  (params (OtherActor :type "Actor Object Reference"))
  (cast `/Game/New_P38/BluePrints/BP_P38_Pawn` OtherActor
    (:`CastFailed`
      (`GameplayStatics.SpawnEmitterAtLocation` "/Game/StarterContent/Particles/P_Explosion.P_Explosion" (`self.K2_GetActorLocation`))
      (`self.K2_DestroyActor`))))

(fn `UserConstructionScript`)